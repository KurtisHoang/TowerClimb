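; BP_EndLevelStar is an end-of-level pickup that reloads the current level when the player's BP_King overlaps it.
; On collision-box overlap it stores and freezes the king, waits a configurable delay, then reopens the current level by name and calls the EndLevel dispatcher.
; The construction script applies a configurable play rate to its Paper2D flipbook.
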(event `self.ReceiveBeginPlay`)

(event `self.ReceiveActorBeginOverlap`
  (params (OtherActor :type "Actor Object Reference")))

(event `self.CollisionBox.OnComponentBeginOverlap`
  (params (OverlappedComponent :type "PrimitiveComponent Object Reference") (OtherActor :type "Actor Object Reference") (OtherComp :type "PrimitiveComponent Object Reference") (OtherBodyIndex :type Integer) (bFromSweep :type Boolean) (SweepResult :type "HitResult Structure (by ref)"))
  (bind _asbp_king (cast `/Game/Dynamic/Blueprints/Characters/King/BP_King` OtherActor))
  (bind _output_get (set `self.Player` _asbp_king))
  (`/Game/Dynamic/Blueprints/Characters/King/BP_King.Freeze` _output_get)
  (`KismetSystemLibrary.Delay` (`self.RestartLevelDelay`))
  (bind _returnvalue (`GameplayStatics.GetCurrentLevelName` true))
  (`GameplayStatics.OpenLevel` (`KismetStringLibrary.Conv_StringToName` _returnvalue))
  (`self.EndLevel`))

(fn `UserConstructionScript`
  (`PaperFlipbookComponent.SetPlayRate` (`self.PaperFlipbook`) (`self.NewPlayRate`)))