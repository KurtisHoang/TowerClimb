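; BP_King is a player-controllable character Blueprint, set up for platformer input but with only placeholder actions.
; On BeginPlay it casts its controller to PlayerController and adds the IMC_Platformer mapping context through the Enhanced Input subsystem.
; The IA_Move and IA_Jump Started events only print debug strings, with no movement or jump logic in this graph.
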(event `self.ReceiveBeginPlay`
  (`parent.ReceiveBeginPlay`)
  (bind _asplayer_controller (cast `PlayerController` (`self.GetController`)))
  (`EnhancedInputSubsystemInterface.AddMappingContext` (pcsubsystem `EnhancedInputLocalPlayerSubsystem` _asplayer_controller) "/Game/Dynamic/Input/IMC_Platformer.IMC_Platformer" 0 (struct)))

(event `EnhancedInput|/Game/Dynamic/Input/Actions/IA_Move`
  (params (ActionValue :type "Float (double-precision)") (ElapsedSeconds :type "Float (double-precision)") (TriggeredSeconds :type "Float (double-precision)") (InputAction :type "InputAction Object Reference" :default "/Game/Dynamic/Input/Actions/IA_Move.IA_Move"))
  (:`Started`
    (`KismetSystemLibrary.PrintString` "Move")))

(event `EnhancedInput|/Game/Dynamic/Input/Actions/IA_Jump`
  (params (ActionValue :type Boolean) (ElapsedSeconds :type "Float (double-precision)") (TriggeredSeconds :type "Float (double-precision)") (InputAction :type "InputAction Object Reference" :default "/Game/Dynamic/Input/Actions/IA_Jump.IA_Jump"))
  (:`Started`
    (`KismetSystemLibrary.PrintString` "Jump")))

(fn `UserConstructionScript`
  (`parent.UserConstructionScript`))